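; Base enemy Blueprint that provides the health bar display and floating damage numbers for enemies.
; On BeginPlay it passes itself to the health bar widget and hides it, with show and hide events toggling visibility afterward.
; Each damage event spawns a damage number widget at the screen-projected hit location, stores it with that location, sets its text and headshot flag, and plays a fade-out animation.
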(event `self.ReceiveBeginPlay`
  (bind _aswbp_enemy_health_bar (cast `/Game/_Game/HUD/WBP_EnemyHealthBar` (`WidgetComponent.GetUserWidgetObject` (`self.HealthBar`))))
  (set `/Game/_Game/HUD/WBP_EnemyHealthBar.EnemyRef` self _aswbp_enemy_health_bar)
  (`Widget.SetVisibility` (`WidgetComponent.GetUserWidgetObject` (`self.HealthBar`)) "Hidden"))

(event `self.ShowHealthBar`
  (`parent.ShowHealthBar`)
  (`Widget.SetVisibility` (`WidgetComponent.GetUserWidgetObject` (`self.HealthBar`)) "Visible"))

(event `self.HideHealthBar`
  (`Widget.SetVisibility` (`WidgetComponent.GetUserWidgetObject` (`self.HealthBar`)) "Hidden"))

(event `self.ShowDamageNumber`
  (params (Damage :type Integer) (HitLocation :type "Vector Structure") (bIsHeadShot :type Boolean))
  (bind _returnvalue (`|CreateWidget` "/Game/_Game/HUD/WBP_DamageNumber.WBP_DamageNumber_C"))
  (`UserWidget.AddToViewport` _returnvalue 0)
  (`UserWidget.SetPositionInViewport` _returnvalue (`GameplayStatics.ProjectWorldToScreen` (`GameplayStatics.GetPlayerController` 0) HitLocation) true)
  (`self.StoreDamageNumber` _returnvalue HitLocation)
  (set `/Game/_Game/HUD/WBP_DamageNumber.DamageText` (`KismetTextLibrary.Conv_IntToText` Damage) _returnvalue)
  (set `/Game/_Game/HUD/WBP_DamageNumber.IsHeadshot` bIsHeadShot _returnvalue)
  (`UserWidget.PlayAnimation` _returnvalue (`/Game/_Game/HUD/WBP_DamageNumber.DamageNumberFadeOut` _returnvalue) 0.0 1 "Forward" 1.0 false))

(fn `UserConstructionScript`)